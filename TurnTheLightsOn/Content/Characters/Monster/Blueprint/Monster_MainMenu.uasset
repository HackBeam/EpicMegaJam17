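; Monster actor, named for the main menu, with functions for screaming and teleporting between TargetPoints; BeginPlay and Tick are empty.
; Construction caches MonsterInitialPosition as WaitPoint for MoveToInitialPosition, and Scream plays once whenever the player comes close.
; MonsterReturn seeks a random point away from the player, but re-rolls between checks and assignment, so the result can fail them.
; ChangeState starts a timer for ReturnState, which clears Death.
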(event `self.ReceiveBeginPlay`)

(event `self.ReceiveTick`
  (params (DeltaSeconds :type "Float (single-precision)")))

(fn `ChangeState`
  (`KismetSystemLibrary.K2_SetTimer` null "ReturnState" 5.0)
  (`KismetSystemLibrary.PrintString` "CAMBIO HECHO"))

(fn `GetWaitPoint`
  (bind _outactors (`GameplayStatics.GetAllActorsOfClass` "/Script/Engine.TargetPoint"))
  (for _array_element _outactors
    (if (`KismetStringLibrary.EqualEqual_StrStr` (`KismetSystemLibrary.GetObjectName` _array_element) "MonsterInitialPosition")
      (set `self.WaitPoint` _array_element))))

(fn `MonsterReturn`
  (locals (notPoint :type Boolean :default true) (Point :type "Actor Object Reference"))
  (bind _point (`local.Point`))
  (if (not (`self.death`))
    (while (`local.notPoint`)
      (bind _outactors (`GameplayStatics.GetAllActorsOfClass` "/Script/Engine.TargetPoint"))
      (bind _output (`|GetArrayItem` _outactors (`KismetMathLibrary.RandomIntegerInRange` 0 (- (`KismetArrayLibrary.Array_Length` _outactors) 1))))
      (if (!= _output (`self.WaitPoint`))
        (if (> (`self.GetDistanceTo` _output (`GameplayStatics.GetPlayerCharacter` 0)) 1000.0)
          (set `local.Point` _output)
          (set `local.notPoint` false))))
    (if (`KismetSystemLibrary.IsValid` _point)
      (`self.K2_SetActorLocation` (`self.K2_GetActorLocation` _point) false true))))

(fn `MoveToInitialPosition`
  (`self.K2_SetActorLocation` (`self.K2_GetActorLocation` (`self.WaitPoint`)) false true))

(fn `ReturnState`
  (`KismetSystemLibrary.PrintString` "ENTRO EN FUNCIÓN")
  (set `self.death` false)
  (`KismetSystemLibrary.PrintString` "ESTADO CAMBIADO"))

(fn `Scream`
  (if (< (`self.GetDistanceTo` (`GameplayStatics.GetPlayerCharacter` 0)) 200.0)
    (if (not (`self.atack`))
      (set `self.atack` true)
      (`GameplayStatics.PlaySoundAtLocation` "/Game/Sounds/MonsterScream.MonsterScream" (`self.K2_GetActorLocation` self)))
    (else
      (set `self.atack` false))))

(fn `UserConstructionScript`
  (`self.GetWaitPoint`))