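; Monster character that waits at a set point, can relocate around the level, and screams when the player comes close.
; BeginPlay finds TargetPoints, parks the scaled-down monster at MonsterInitialPosition and flags it dead; the others become appearance points.
; Tick plays a scream once per entry within range.
; MonsterReturn, if not dead, teleports it to a random point, re-rolled after the far-from-player check; ChangeState schedules ReturnState, undefined here.
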(event `self.ReceiveBeginPlay`
  (`self.GetWaitPoint`)
  (`self.GetApperationPoints`)
  (`self.MoveToInitialPosition`))

(event `self.ReceiveTick`
  (params (DeltaSeconds :type "Float (single-precision)"))
  (`self.Scream`))

(fn `ChangeState`
  (`KismetSystemLibrary.K2_SetTimer` null "ReturnState" 5.0))

(fn `GetApperationPoints`
  (bind _outactors (`GameplayStatics.GetAllActorsOfClass` "/Script/Engine.TargetPoint"))
  (bind _output_get (set `self.ApperationPoints` _outactors))
  (`KismetArrayLibrary.Array_RemoveItem` _output_get (`self.WaitPoint`)))

(fn `GetBigger`
  (params (Size :type "Vector Structure"))
  (`self.SetActorScale3D` Size))

(fn `GetSmall`
  (params (Size :type "Vector Structure"))
  (`self.SetActorScale3D` Size))

(fn `GetWaitPoint`
  (bind _outactors (`GameplayStatics.GetAllActorsOfClass` "/Script/Engine.TargetPoint"))
  (for _array_element _outactors
    (if (`KismetStringLibrary.EqualEqual_StrStr` (`KismetSystemLibrary.GetObjectName` _array_element) "MonsterInitialPosition")
      (set `self.WaitPoint` _array_element))))

(fn `MonsterReturn`
  (locals (notPoint :type Boolean :default true) (Point :type "Actor Object Reference"))
  (bind _apperationpoints (`self.ApperationPoints`))
  (bind _point (`local.Point`))
  (bind _output (`|GetArrayItem` _apperationpoints (`KismetMathLibrary.RandomIntegerInRange` 0 (- (`KismetArrayLibrary.Array_Length` _apperationpoints) 1))))
  (if (not (`self.death`))
    (while (`local.notPoint`)
      (if (> (`self.GetDistanceTo` _output (`GameplayStatics.GetPlayerCharacter` 0)) 1000.0)
        (set `local.Point` _output)
        (set `local.notPoint` false)))
    (if (`KismetSystemLibrary.IsValid` _point)
      (`self.K2_SetActorLocation` (`self.K2_GetActorLocation` _point) false true))))

(fn `MoveToInitialPosition`
  (`self.GetBigger` (0.75 0.75 0.75))
  (`self.K2_SetActorLocation` (`self.K2_GetActorLocation` (`self.WaitPoint`)) false true)
  (set `self.death` true))

(fn `Scream`
  (if (< (`self.GetDistanceTo` (`GameplayStatics.GetPlayerCharacter` 0)) 200.0)
    (if (not (`self.atack`))
      (set `self.atack` true)
      (`GameplayStatics.PlaySoundAtLocation` "/Game/Sounds/MonsterScream.MonsterScream" (`self.K2_GetActorLocation` self)))
    (else
      (set `self.atack` false))))

(fn `UserConstructionScript`)