(fn `actionUnlocked`)

(fn `unlock`
  (if (not (`self.unlocked`))
    (bind _outactors (`GameplayStatics.GetAllActorsOfClass` "/Game/Blueprints/Inventory.Inventory_C"))
    (bind _output (`|GetArrayItem` _outactors))
    (bind _items (`/Game/Blueprints/Inventory.Items` _output))
    (if (== (`KismetArrayLibrary.Array_Length` _items) 0)
      (`KismetSystemLibrary.PrintString` "No tienes el objeto" :!label _label)
      (else
        (for _array_element _items
          (if (== (`GameplayStatics.GetObjectClass` _array_element) (`self.itemNeeded`))
            (`/Game/Blueprints/Inventory.useItem` _output _array_element)
            (set `self.unlocked` true)
            (`self.actionUnlocked`)
            (else
              (goto _label))))))))

(fn `UserConstructionScript`)