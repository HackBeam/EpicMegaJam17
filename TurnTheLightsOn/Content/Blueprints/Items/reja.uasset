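; Gate actor (reja) that rises when a Monster overlaps its Colision component while closed, then lowers after a short delay.
; The overlap fires the open event and calls GetSmall on the monster with a half-size vector.
; The MoveUp timeline offsets Z from the height saved at BeginPlay, scaled by Height, and plays in reverse to close.
; An Opened flag blocks retriggering until closing starts.
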(event `self.ReceiveBeginPlay`
  (bind (_returnvalue_x _returnvalue_y _returnvalue_z) (`KismetMathLibrary.BreakVector` (`self.K2_GetActorLocation`)))
  (set `self.initialZ` _returnvalue_z))

(event `OpenTickRecieved`
  (bind (_returnvalue_x _returnvalue_y) (`KismetMathLibrary.BreakVector` (`self.K2_GetActorLocation`)))
  (set `self.opened` true)
  (bind (_direction _z) (`Timeline|MoveUp` :!via `PlayFromStart` :!label _label)
    (:`Update`
      (`self.K2_SetActorRelativeLocation` (`KismetMathLibrary.MakeVector` _returnvalue_x _returnvalue_y (+ (* _z (`self.height`)) (`self.initialZ`)))))))

(event `CloseTickRecieved`
  (set `self.opened` false)
  (goto _label :!via `ReverseFromEnd`))

(event `self.Colision.OnComponentBeginOverlap`
  (params (OverlappedComponent :type "PrimitiveComponent Object Reference") (OtherActor :type "Actor Object Reference") (OtherComp :type "PrimitiveComponent Object Reference") (OtherBodyIndex :type Integer) (bFromSweep :type Boolean) (SweepResult :type "HitResult Structure (by ref)"))
  (if (and (`KismetMathLibrary.ClassIsChildOf` (`GameplayStatics.GetObjectClass` OtherActor) "/Game/Characters/Monster/Blueprint/Monster.Monster_C") (== (`self.opened`) false))
    (`self.OpenTickRecieved`)
    (bind _asmonster (cast `/Game/Characters/Monster/Blueprint/Monster` OtherActor))
    (`/Game/Characters/Monster/Blueprint/Monster.GetSmall` _asmonster (0.5 0.5 0.5))
    (`KismetSystemLibrary.Delay` 3.0)
    (`self.CloseTickRecieved`)))

(fn `UserConstructionScript`)