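; BP_Generador_OBSOLETO is a generator, marked obsolete by name, that restores tagged lights and opens an iron door when turned on.
; Its construction script caches every actor tagged GeneratorLights and the first BP_PuertasHierro found in the level.
; SwitchLights toggles each light component's visibility, running at BeginPlay to switch them off.
; TurnOnGenerator toggles them again and calls Open on the door.
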(event `self.ReceiveBeginPlay`
  ;[1 1 1] Switch Off
  (`self.SwitchLights`))

(fn `SwitchLights`
  (for _array_element (`self.Lights`)
    (bind _aslight (cast `Light` _array_element))
    (`SceneComponent.ToggleVisibility` (`Light.LightComponent` _aslight) false)))

(fn `TurnOnGenerator`
  (`self.SwitchLights`)
  (`/Game/Blueprints/BP_PuertasHierro.Open` (`self.Door`)))

(fn `UserConstructionScript`
  (bind _outactors (`GameplayStatics.GetAllActorsWithTag` "GeneratorLights"))
  (set `self.Lights` _outactors)
  (bind _outactors_2 (`GameplayStatics.GetAllActorsOfClass` "/Game/Blueprints/BP_PuertasHierro.BP_PuertasHierro_C"))
  (set `self.Door` (`|GetArrayItem` _outactors_2)))