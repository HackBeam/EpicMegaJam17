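; Lever item that temporarily opens the level's gate (Reja) when activated.
; Activate clears the Active flag, rotates the cylinder with a timeline, then tells the first Reja actor found to open and starts a fixed timer.
; The timer runs Deactivate, which tells the gate to close, rotates the cylinder with a second timeline and sets Active again once that finishes.
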(event `self.activate`
  (set `self.active` false)
  (bind (_direction _rotation) (`Timeline|GoDown` :!via `PlayFromStart`)
    (:`Update`
      (`SceneComponent.K2_SetRelativeRotation` (`self.Cylinder`) (`KismetMathLibrary.MakeRotator` _rotation) false false))
    (:`Finished`
      (bind _outactors (`GameplayStatics.GetAllActorsOfClass` "/Game/Blueprints/Items/reja.reja_C"))
      (`/Game/Blueprints/Items/reja.OpenTickRecieved` (`|GetArrayItem` _outactors))
      (`KismetSystemLibrary.K2_SetTimer` null "deactivate" 5.0))))

(event `self.deactivate`
  (bind _outactors (`GameplayStatics.GetAllActorsOfClass` "/Game/Blueprints/Items/reja.reja_C"))
  (`/Game/Blueprints/Items/reja.CloseTickRecieved` (`|GetArrayItem` _outactors))
  (bind (_direction _rotation) (`Timeline|GoUp` :!via `PlayFromStart`)
    (:`Update`
      (`SceneComponent.K2_SetRelativeRotation` (`self.Cylinder`) (`KismetMathLibrary.MakeRotator` _rotation) false false))
    (:`Finished`
      (set `self.active` true))))

(fn `UserConstructionScript`
  (`parent.UserConstructionScript`))