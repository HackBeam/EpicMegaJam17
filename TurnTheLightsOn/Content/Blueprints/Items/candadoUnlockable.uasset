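; Padlock unlockable that requires a key (LlaveItem) and enables the BidonItem pickups once unlocked.
; The construction script sets LlaveItem as the needed item on the inherited unlockable logic.
; On ActionUnlocked it waits briefly, then finds every BidonItem actor in the level and sets it active.
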(event `self.actionUnlocked`
  (`KismetSystemLibrary.Delay` 2.0)
  (bind _outactors (`GameplayStatics.GetAllActorsOfClass` "/Game/Blueprints/Items/bidonItem.bidonItem_C"))
  (for _array_element _outactors
    (set `/Game/Blueprints/Item.active` true _array_element)))

(fn `UserConstructionScript`
  (`parent.UserConstructionScript`)
  (set `self.itemNeeded` "/Game/Blueprints/Items/llaveItem.llaveItem_C"))