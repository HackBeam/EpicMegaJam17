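; Starting door item (puertaInicio) that swings open or closed on activation and opens automatically when a Monster enters its trigger box.
; Activate plays or reverses the Open timeline to yaw the Pivot, with an Active flag blocking re-triggering until it finishes and flips Opened.
; Any Monster overlapping the Box also receives a GetSmall call with a fixed uniform vector, apparently to shrink it.
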(event `self.activate`
  (bind _opened (`self.opened`))
  (if (`self.active`)
    (set `self.active` false)
    (if _opened
      (bind (_direction _rotationz) (`Timeline|Open` :!via `ReverseFromEnd` :!label _label)
        (:`Update`
          (`SceneComponent.K2_SetRelativeRotation` (`self.pivot`) (`KismetMathLibrary.MakeRotator` 0.0 0.0 _rotationz) false false))
        (:`Finished`
          (set `self.opened` (not _opened))
          (set `self.active` true)))
      (else
        (goto _label :!via `PlayFromStart`)))))

(event `self.Box.OnComponentBeginOverlap`
  (params (OverlappedComponent :type "PrimitiveComponent Object Reference") (OtherActor :type "Actor Object Reference") (OtherComp :type "PrimitiveComponent Object Reference") (OtherBodyIndex :type Integer) (bFromSweep :type Boolean) (SweepResult :type "HitResult Structure (by ref)"))
  (bind _returnvalue (`KismetMathLibrary.ClassIsChildOf` (`GameplayStatics.GetObjectClass` OtherActor) "/Game/Characters/Monster/Blueprint/Monster.Monster_C"))
  (if (and _returnvalue (== (`self.opened`) false))
    (`self.activate`))
  (if _returnvalue
    (bind _asmonster (cast `/Game/Characters/Monster/Blueprint/Monster` OtherActor))
    (`/Game/Characters/Monster/Blueprint/Monster.GetSmall` _asmonster (0.35 0.35 0.35))))

(fn `UserConstructionScript`
  (`parent.UserConstructionScript`))