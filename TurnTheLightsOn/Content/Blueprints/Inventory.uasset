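; Inventory actor that stores items and displays them at physical ItemPosition slots in the level, viewed through a dedicated camera.
; The Construction Script caches all ItemPosition actors and the camera tagged InventoryCamera.
; AddItem records every item, but only picks it up and moves it when an empty slot exists.
; UseItem removes and destroys held items, while SwitchCamera toggles the view between pawn and inventory camera.
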(event `self.ReceiveBeginPlay`)

(fn `addItem`
  (params (item :type "/Game/Blueprints/Item Object Reference"))
  (`KismetArrayLibrary.Array_Add` (`self.Items`) item)
  (bind _position (`self.findEmptyPosition`))
  (if (`KismetSystemLibrary.IsValid` _position)
    (`self.useEmptyPosition` _position item)
    (`/Game/Blueprints/Item.PickUp` item)))

(fn `findEmptyPosition`
  (returns (Position :type "/Game/Blueprints/ItemPosition Object Reference"))
  (locals (Pos :type "/Game/Blueprints/ItemPosition Object Reference"))
  (for _array_element (`self.Positions`)
    (if (== (`/Game/Blueprints/ItemPosition.Empty` _array_element) true)
      (set `local.Pos` _array_element)
      (break)))
  (return (`local.Pos`)))

(fn `removeItem`
  (params (Item :type "/Game/Blueprints/Item Object Reference"))
  (`KismetArrayLibrary.Array_RemoveItem` (`self.Items`) Item)
  (`/Game/Blueprints/Item.DestroyItem` Item))

(fn `SwitchCamera`
  (bind _returnvalue (`GameplayStatics.GetPlayerController` 0))
  (if (`self.cameraSwitched`)
    (`PlayerController.SetViewTargetWithBlend` _returnvalue (`Controller.K2_GetPawn` _returnvalue) 0.0 "VTBlend_EaseInOut" 1.0 true)
    (set `self.cameraSwitched` false)
    (else
      (`PlayerController.SetViewTargetWithBlend` (`GameplayStatics.GetPlayerController` 0) (`self.Camera`) 0.0 "VTBlend_EaseInOut" 1.0 true)
      (set `self.cameraSwitched` true))))

(fn `useEmptyPosition`
  (params (Pos :type "/Game/Blueprints/ItemPosition Object Reference") (Item :type "/Game/Blueprints/Item Object Reference"))
  (bind _output_get (set `/Game/Blueprints/Item.Position` Pos Item))
  (set `/Game/Blueprints/ItemPosition.Empty` false _output_get)
  (`/Game/Blueprints/Item.MoveToInventory` Item))

(fn `useItem`
  (params (Item :type "/Game/Blueprints/Item Object Reference"))
  (returns (Success :type Boolean))
  (bind _returnvalue (!= (`KismetArrayLibrary.Array_Find` (`self.Items`) Item) -1))
  (if _returnvalue
    (`self.removeItem` Item))
  (return _returnvalue))

(fn `UserConstructionScript`
  (bind _outactors (`GameplayStatics.GetAllActorsOfClass` "/Game/Blueprints/ItemPosition.ItemPosition_C"))
  (set `self.Positions` _outactors)
  (bind _outactors_2 (`GameplayStatics.GetAllActorsWithTag` "InventoryCamera"))
  (bind _ascamera_actor (cast `CameraActor` (`|GetArrayItem` _outactors_2)))
  (set `self.Camera` _ascamera_actor))