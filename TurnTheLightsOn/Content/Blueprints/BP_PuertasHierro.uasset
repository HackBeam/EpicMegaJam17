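; BP_PuertasHierro is an iron double door whose two leaves slide open when its Open event is called.
; The construction script stores the starting world location of each leaf.
; Open plays the Puertas timeline, whose per-leaf tracks are added to those stored locations every update to move the leaves without sweep.
; The offsets apply in world space, and the Blueprint has no closing logic or trigger of its own.
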(event `self.ReceiveBeginPlay`)

(event `Open`
  (bind (_direction _puertader _puertaizq) (`Timeline|Puertas`)
    (:`Update`
      (`SceneComponent.K2_SetWorldLocation` (`self.PuertaDer`) (+ _puertader (`self.PuertaDerPosInicial`)) false false)
      (`SceneComponent.K2_SetWorldLocation` (`self.PuertaIzq`) (+ _puertaizq (`self.PuertaIzqPosInicial`)) false false))))

(fn `UserConstructionScript`
  (set `self.PuertaDerPosInicial` (`SceneComponent.K2_GetComponentLocation` (`self.PuertaDer`)))
  (set `self.PuertaIzqPosInicial` (`SceneComponent.K2_GetComponentLocation` (`self.PuertaIzq`))))