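; Clock actor that acts as the game's visible timer, signalling the player character when the time limit nears and expires.
; Tick accumulates time while unpaused and yaws two hand pivots; despite their names, MinutesAxis sweeps as seconds and HourAxis as minutes.
; Sixty seconds before MAXTIME it sets LastMinute on itself and the FirstPersonCharacter, then sets the character's LightsOut once MAXTIME is reached.
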(event `self.ReceiveTick`
  (params (DeltaSeconds :type "Float (single-precision)"))
  (bind _returnvalue (`GameplayStatics.GetPlayerPawn` 0))
  (if (not (`GameplayStatics.IsGamePaused`))
    (bind _output_get (set `self.Time` (+ DeltaSeconds (`self.Time`))))
    ;[1 1 1] Multiplicar por 6 para los segundos y por 0.1 para los minutos (para horas 0.008333, pero no tenemos manecilla de horas)
    (`SceneComponent.K2_SetRelativeRotation` (`self.hourAxis`) (`KismetMathLibrary.MakeRotator` 0.0 0.0 (* _output_get 0.1)) false false)
    (`SceneComponent.K2_SetRelativeRotation` (`self.minutesAxis`) (`KismetMathLibrary.MakeRotator` 0.0 0.0 (* _output_get 6.0)) false false)
    (if (>= (`self.Time`) (- (`self.MAXTIME`) 60.0))
      (if (`self.lastMinute`)
        (if (>= (`self.Time`) (`self.MAXTIME`))
          (bind _asfirst_person_character (cast `/Game/Blueprints/FirstPersonCharacter` _returnvalue))
          (set `/Game/Blueprints/FirstPersonCharacter.lightsOut` true _asfirst_person_character))
        (else
          (set `self.lastMinute` true)
          (bind _asfirst_person_character_2 (cast `/Game/Blueprints/FirstPersonCharacter` _returnvalue))
          (set `/Game/Blueprints/FirstPersonCharacter.lastMinute` true _asfirst_person_character_2))))))

(fn `UserConstructionScript`)